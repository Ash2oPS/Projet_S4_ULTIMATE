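; Painting actor (Papi Cri) whose material blend gradually changes while it is looked at, once the "Jour2" global flag is true.
; The construction script creates a dynamic material instance and measures the mesh's world size.
; Tick accumulates capped time while IsLooking, which is set outside this graph, drains it twice as fast otherwise, and feeds BlendParameter.
; An older camera-angle facing test that scaled heat-haze distortion remains disconnected, along with its debug prints.
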(event EventBeginPlay)

(event Collision|EventActorBeginOverlap
  (params (OtherActor :type Actor%20Object%20Reference)))

(event EventTick
  (params (DeltaSeconds :type Float%20%28single-precision%29))
  (bind _returnvalue (Utilities|Time|GetWorldDeltaSeconds))
  (bind _asbp_global_variables (Utilities|Casting|CastToBP_GlobalVariables (CallFunction|GetGlobalVariables)))
  (if (Default|GetBoolValue _asbp_global_variables (Utilities|String|MakeLiteralString "Jour2"))
    (if (Variables|Default|GetisLooking)
      (Variables|Default|SetAccumulativeMethodeValue (Math|Float|Min(Float) (+ (Variables|Default|GetAccumulativeMethodeValue) _returnvalue) (Variables|Default|GetMaxAccumulativeMethodeValue)))
      (else
        (Variables|Default|SetAccumulativeMethodeValue (Math|Float|Max(Float) (+ (Variables|Default|GetAccumulativeMethodeValue) (* _returnvalue -2.0)) 0.0))))
    (Rendering|Material|SetScalarParameterValue (Variables|Default|GetInstanceHeatHaze) "BlendParameter" (Variables|Default|GetAccumulativeMethodeValue) :!class /Script/Engine.MaterialInstanceDynamic)))

(event Input|ActionEvents|InputActionInteract
  (params (Key :type Key%20Structure :default "None")))

(fn ConstructionScript
  (bind _self self)
  (bind _staticmeshcomponent (Variables|Debug|GetStaticMeshComponent))
  (bind (_min _max) (Components|StaticMesh|GetLocalBounds _staticmeshcomponent))
  (bind _staticmeshcomponent_2 (Variables|Debug|GetStaticMeshComponent _self))
  (bind _returnvalue (- _max _min))
  (bind _returnvalue_2 (Transformation|GetWorldScale _staticmeshcomponent_2))
  (bind _returnvalue_3 (Rendering|Material|CreateDynamicMaterialInstance (Variables|Debug|GetStaticMeshComponent) 0 "/Game/Materials/VFX/HeatDeformation/PAPI_CRI_Mat_Inst.PAPI_CRI_Mat_Inst" "None" :!class /Script/Engine.PrimitiveComponent))
  (bind _output_get (Variables|Default|SetInstanceHeatHaze _returnvalue_3))
  (Rendering|Material|SetMaterial (Variables|Debug|GetStaticMeshComponent) 0 _output_get)
  (Variables|Default|SetlargeurObjetReelle (* (.x _returnvalue) (.x _returnvalue_2)))
  (Variables|Default|SethauteurObjetReelle (* (.y _returnvalue) (.y _returnvalue_2))))

(fn AngleBetweenVectors
  (params (VectorA :type Vector) (VectorB :type Vector))
  (return (Class|KismetMathLibrary|DegAcos (Math|Vector|DotProduct (Math|Vector|Normalize VectorA) (Math|Vector|Normalize VectorB)))))

(fn CalculeAngle
  (params (TailleReelle :type Float%20%28single-precision%29))
  (return (* (/ TailleReelle (Math|Vector|VectorLength (- (Transformation|GetActorLocation self) (Transformation|GetWorldLocation (Variables|/Game/BP/Character/BP_Player.BP_Player_C|GetFirstPersonCamera (CallFunction|GetMyCharacter)))))) (Variables|Default|GetConstanteRapportDistance))))

(fn CalculDifferenceAngles
  (bind _playercharacter (CallFunction|GetMyCharacter))
  (bind _self self)
  (bind _returnvalue (Transformation|GetActorLocation _self))
  (bind _firstpersoncamera (Variables|/Game/BP/Character/BP_Player.BP_Player_C|GetFirstPersonCamera _playercharacter))
  (bind _returnvalue_2 (Transformation|GetWorldRotation _firstpersoncamera))
  (bind _returnvalue_3 (Transformation|GetWorldLocation _firstpersoncamera))
  (bind _returnvalue_4 (- _returnvalue _returnvalue_3))
  (bind _returnvalue_5 (Math|Rotator|GetRotationXVector _returnvalue_2))
  (return (CallFunction|AngleBetweenVectors (Math|Vector|MakeVector (Math|Float|Sqrt (+ (Math|Float|Power (.x _returnvalue_4) 2.0) (Math|Float|Power (.y _returnvalue_4) 2.0))) 0.0 (.z _returnvalue_4)) (Math|Vector|MakeVector (Math|Float|Sqrt (+ (Math|Float|Power (.x _returnvalue_5) 2.0) (Math|Float|Power (.y _returnvalue_5) 2.0))) 0.0 (.z _returnvalue_5))) (CallFunction|AngleBetweenVectors (Math|Vector|MakeVector (.x _returnvalue_4) (.y _returnvalue_4) 0.0) (Math|Vector|MakeVector (.x _returnvalue_5) (.y _returnvalue_5) 0.0))))