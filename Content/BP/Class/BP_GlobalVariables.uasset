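; BP_GlobalVariables is a key-value store for global bool and int variables, kept in two maps with a setter and getter for each type.
; Setters add or overwrite entries, while getters look up the key and, on failure, print an error and return false or zero.
; GetBoolValue branches on the stored value instead of the found flag, so a stored false also triggers the missing-key error.
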(fn SetBoolValue
  (params (Key :type String%20%28by%20ref%29) (Value :type Boolean%20%28by%20ref%29))
  (Utilities|Map|Add (Variables|Default|GetBoolVariables) Key Value))

(fn GetBoolValue
  (params (Key :type String%20%28by%20ref%29))
  (bind _boolvariables (Variables|Default|GetBoolVariables))
  (bind (_value _returnvalue) (Utilities|Map|Find _boolvariables Key))
  (if _value
    (return _returnvalue)
    (else
      (Development|PrintString (Variables|Default|GetParent) (Utilities|String|Append "ERROR The value related to the key " Key " has not been found. The default value has been returned"))
      (return false))))

(fn SetIntValue
  (params (Key :type String%20%28by%20ref%29) (Value :type Integer%20%28by%20ref%29))
  (Utilities|Map|Add (Variables|Default|GetIntVariables) Key Value))

(fn GetIntValue
  (params (Key :type String%20%28by%20ref%29))
  (bind _intvariables (Variables|Default|GetIntVariables))
  (bind (_value _returnvalue) (Utilities|Map|Find _intvariables Key))
  (if _returnvalue
    (return _value)
    (else
      (Development|PrintString (Variables|Default|GetParent) (Utilities|String|Append "ERROR The value related to the key " Key " has not been found. The default value has been returned"))
      (return 0))))