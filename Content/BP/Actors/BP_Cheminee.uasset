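; BP_Cheminee is a fireplace actor whose fire can be switched on and off.
; EnableFire and DisableFire toggle each fire particle, the audio and the FireIsOn flag, with disabling also zeroing the point light.
; FireAnim, also run at BeginPlay if lit, flickers the light through a self-restarting timeline scaled by a maximum intensity.
; DisableFire never stops that timeline, so a running flicker keeps overwriting the zeroed intensity.
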(event Custom|DisableFire
  (Variables|Default|SetFireIsOn false)
  (for _array_element (Variables|Default|GetFireParticle)
    (Variables|/Game/Particles_Wind_Control_System/Blueprints/BP_Particle_Candle_Fire.BP_Particle_Candle_Fire_C|SetFire%20Enabled _array_element false)
    (Audio|Components|Audio|Stop (Variables|Default|GetAudio))
    (Rendering|Components|Light|SetIntensity (Variables|Default|GetPointLight) 0.0)))

(event Custom|FireAnim
  (bind _lightpower (Timeline|LightFlickering Play)
    (:Update
      (Variables|Default|SetLightIntensity (* _lightpower (Variables|Default|GetLightMaxIntensity)))
      (Rendering|Components|Light|SetIntensity (Variables|Default|GetPointLight) (Variables|Default|GetLightIntensity)))
    (:Finished
      (CallFunction|FireAnim))))

(event Custom|EnableFire
  (Variables|Default|SetFireIsOn true)
  (for _array_element (Variables|Default|GetFireParticle)
    (Variables|/Game/Particles_Wind_Control_System/Blueprints/BP_Particle_Candle_Fire.BP_Particle_Candle_Fire_C|SetFire%20Enabled _array_element true)
    (Audio|Components|Audio|Play (Variables|Default|GetAudio) 0.0)
    (CallFunction|FireAnim)))

(event EventBeginPlay
  (if (Variables|Default|GetFireIsOn)
    (CallFunction|FireAnim)))

(fn ConstructionScript)