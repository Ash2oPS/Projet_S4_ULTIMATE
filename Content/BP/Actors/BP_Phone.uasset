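; BP_Phone is a phone actor that can be switched between ringing and silent states.
; RingtoneOn starts the vibration and ringtone audio, swaps a material slot on the phone mesh to MatOn and lights a spotlight.
; RingtoneOff stops both sounds, applies MatOff and sets the light's intensity to zero.
; Nothing in its graphs triggers either event.
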(event Custom|RingtoneOn
  (Audio|Components|Audio|Play (Variables|Default|GetAudioVibreur) 0.0)
  (Audio|Components|Audio|Play (Variables|Default|GetAudioRingtone) 0.0)
  (Rendering|Material|SetMaterial (Variables|Default|GetSM_Phone) 1 (Variables|Default|GetMatOn))
  (Rendering|Components|Light|SetIntensity (Variables|Default|GetSpotLight) 7e+03))

(event Custom|RingtoneOff
  (Audio|Components|Audio|Stop (Variables|Default|GetAudioVibreur))
  (Audio|Components|Audio|Stop (Variables|Default|GetAudioRingtone))
  (Rendering|Material|SetMaterial (Variables|Default|GetSM_Phone) 1 (Variables|Default|GetMatOff))
  (Rendering|Components|Light|SetIntensity (Variables|Default|GetSpotLight) 0.0))

(fn ConstructionScript)