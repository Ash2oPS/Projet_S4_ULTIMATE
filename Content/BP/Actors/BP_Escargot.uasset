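; BP_Escargot is a snail (escargot) actor that can be shown or hidden through its spawned state.
; SetSpawned(true) needs a valid Manager: it registers the EscargotID as visible, shows and plays the looping skeletal mesh animation, and lights the point light for gold snails.
; SetSpawned(false) hides the mesh, stops the animation and turns the light off, without notifying the Manager.
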(event Custom|SetSpawned
  (params (value :type Boolean))
  (bind _skeletalmesh (Variables|Default|GetSkeletalMesh))
  (if value
    (Utilities|IsValid (Variables|Default|GetManager)
      (:Is%20Valid
        (Default|AddEscargottoVisibles (Variables|Default|GetManager) (Variables|Default|GetEscargotID))
        (Rendering|SetVisibility _skeletalmesh true false)
        (Audio|Components|Audio|Play _skeletalmesh true)
        (Variables|Default|Setspawned true)
        (if (Variables|Default|GetGold)
          (Rendering|Components|Light|SetIntensity (Variables|Default|GetPointLight) 1.5e+03))))
    (else
      (Rendering|SetVisibility (Variables|Default|GetSkeletalMesh) false false)
      (Audio|Components|Audio|Stop (Variables|Default|GetSkeletalMesh))
      (Variables|Default|Setspawned false)
      (Rendering|Components|Light|SetIntensity (Variables|Default|GetPointLight) 0.0))))

(fn ConstructionScript)