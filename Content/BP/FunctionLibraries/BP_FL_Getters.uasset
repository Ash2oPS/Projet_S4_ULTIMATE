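; Blueprint function library of global getters for the local player and shared game state.
; GetMyCharacter and GetMyController cast player index 0's character and controller to BP_Player and BP_PC_MainPlayerController.
; GetGlobalVariables casts the game mode to BP_FirstPersonGameMode and returns its GlobaleVariables.
; Each getter hides the lookup and cast, returning a value only when the cast succeeds.
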(fn GetMyCharacter
  (bind _asbp_player (Utilities|Casting|CastToBP_Player (Game|GetPlayerCharacter 0)))
  (return _asbp_player))

(fn GetMyController
  (bind _asbp_pc_main_player_controller (Utilities|Casting|CastToBP_PC_MainPlayerController (Game|GetPlayerController 0)))
  (return _asbp_pc_main_player_controller))

(fn GetGlobalVariables
  (bind _asbp_first_person_game_mode (Utilities|Casting|CastToBP_FirstPersonGameMode (Game|GetGameMode)))
  (return (Variables|/Game/UE_Base/FirstPersonBP/Blueprints/BP_FirstPersonGameMode.BP_FirstPersonGameMode_C|GetGlobaleVariables _asbp_first_person_game_mode)))