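; Blueprint function library that gives gameplay code one-call access to HUD subtitles, info messages and objectives.
; Each function gets the player controller through GetMyController and forwards to one of its widgets.
; Subtitle and info calls show or hide text on InteractUI, with subtitles prefixed by the speaking character's enum name and given a duration.
; Objective calls add, edit or remove indexed entries on the ObjectifsHUD held by BPACHUD.
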(fn CallSubtitles
  (params (Sentence :type Text) (Duration :type Float%20%28single-precision%29) (TalkingCharacter :type BP_E_Characters%20Enum :default "NewEnumerator0"))
  (LocalVariables|SetShownText (Utilities|Text|FormatText "- {Character} -  
{Sentence}" (Utilities|String|EnumtoString TalkingCharacter) Sentence))
  (Default|EditSubtitlesText (Variables|/Game/BP/Manager/BP_PC_MainPlayerController.BP_PC_MainPlayerController_C|GetInteractUI (CallFunction|GetMyController)) (LocalVariables|GetShownText) Duration))

(fn CallInfos
  (params (Info :type Text))
  (bind _output_get (LocalVariables|SetShownText Info))
  (Default|EditInfosText (Variables|/Game/BP/Manager/BP_PC_MainPlayerController.BP_PC_MainPlayerController_C|GetInteractUI (CallFunction|GetMyController)) _output_get))

(fn RemoveInfos
  (Default|HideInfos (Variables|/Game/BP/Manager/BP_PC_MainPlayerController.BP_PC_MainPlayerController_C|GetInteractUI (CallFunction|GetMyController))))

(fn RemoveSubtitles
  (Default|DisabledSubtitle (Variables|/Game/BP/Manager/BP_PC_MainPlayerController.BP_PC_MainPlayerController_C|GetInteractUI (CallFunction|GetMyController))))

(fn NewObjectif
  (params (Text :type Text) (Index :type Integer))
  (Default|NewText (Variables|/Game/BP/Components/ActorComponents/BP_AC_HUD.BP_AC_HUD_C|GetObjectifs_HUD (Variables|/Game/BP/Manager/BP_PC_MainPlayerController.BP_PC_MainPlayerController_C|GetBP_AC_HUD (CallFunction|GetMyController))) Index Text))

(fn EditObjectif
  (params (Text :type Text) (Index :type Integer))
  (Default|EditText (Variables|/Game/BP/Components/ActorComponents/BP_AC_HUD.BP_AC_HUD_C|GetObjectifs_HUD (Variables|/Game/BP/Manager/BP_PC_MainPlayerController.BP_PC_MainPlayerController_C|GetBP_AC_HUD (CallFunction|GetMyController))) Index Text))

(fn RemoveObjectif
  (params (Index :type Integer))
  (Default|RemoveText (Variables|/Game/BP/Components/ActorComponents/BP_AC_HUD.BP_AC_HUD_C|GetObjectifs_HUD (Variables|/Game/BP/Manager/BP_PC_MainPlayerController.BP_PC_MainPlayerController_C|GetBP_AC_HUD (CallFunction|GetMyController))) Index))