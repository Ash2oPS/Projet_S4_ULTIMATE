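; Interactive item Blueprint that the player can select to show an info message and interact with, optionally playing a sound.
; It extends a parent event class, toggling the player controller's raycasting as the player enters or leaves the trigger.
; Selection shows the message, while unselection or destruction removes it and clears the controller's selected object.
; The construction script sizes and positions the interaction box, which is visible in game only in debug mode.
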(event OnComponentEndOverlap(TriggerBox)
  (params (OverlappedComponent :type Primitive%20Component%20Object%20Reference) (OtherActor :type Actor%20Object%20Reference) (OtherComp :type Primitive%20Component%20Object%20Reference) (OtherBodyIndex :type Integer))
  (bind _playercontroller (CallFunction|GetMyController))
  (Utilities|Casting|CastToBP_Player OtherActor)
  (Utilities|IsValid _playercontroller
    (:Is%20Valid
      (Default|SetHastoRaycast _playercontroller false))))

(event Custom|OnSelected
  (Utilities|FlowControl|Sequence
    (:then_0
      (Utilities|IsValid (Variables|Default|GetPlayerController)
        (:Is%20Not%20Valid
          (Variables|Default|SetPlayerController (CallFunction|GetMyController)))))
    (:then_1
      (CallFunction|CallInfos (Variables|Interaction|GetMessage)))))

(event Custom|OnUnselected
  (Utilities|IsValid (Variables|Default|GetPlayerController)
    (:Is%20Valid
      (CallFunction|RemoveInfos)
      (Utilities|IsValid (Variables|/Game/BP/Manager/BP_PC_MainPlayerController.BP_PC_MainPlayerController_C|GetSelectedObject (Variables|Default|GetPlayerController))
        (:Is%20Valid
          (Variables|/Game/BP/Manager/BP_PC_MainPlayerController.BP_PC_MainPlayerController_C|SetSelectedObject (Variables|Default|GetPlayerController) 0))))))

(event Custom|Interaction
  (|CallParentFunction)
  (Utilities|IsValid (Variables|Default|GetSoundToPlay)
    (:Is%20Valid
      (CallFunction|MyPlaySound (Variables|Default|GetSoundToPlay)))))

(event Custom|OnDestruction
  (CallFunction|OnUnselected)
  (Actor|DestroyActor))

(event Custom|insideBoxEdition
  (bind _interactionbox (Variables|Default|GetInteractionBox))
  (bind _insideboxposition (Variables|Box|GetInsideBoxPosition))
  (Components|Box|SetBoxExtent _interactionbox (Variables|Box|GetInsideBoxScale) true)
  (Transformation|SetRelativeLocation _interactionbox (Math|Vector|MakeVector (.x _insideboxposition) (.y _insideboxposition) (+ (.z (Variables|Box|GetInsideBoxScale)) (.z _insideboxposition))) false false))

(event EventPlayerinTrigger
  (Default|SetHastoRaycast (CallFunction|GetMyController) true))

(event EventSetDebug
  (|CallParentFunction)
  (Development|SetHiddeninGame (Variables|Default|GetInteractionBox) (not (Variables|Default|GetDebugMode)) false))

(fn ConstructionScript
  (|CallParentFunction)
  (CallFunction|InsideBoxEdition)
  (CallFunction|SetDebug))

(fn MyPlaySound
  (params (Sound :type Sound%20Wave%20Object%20Reference))
  (Audio|PlaySoundatLocation Sound (Transformation|GetWorldLocation (Variables|Default|GetInteractionBox)) "0, 0, 0" 1.0 1.0 0.0 (Variables|Default|GetSoundAttenuation) 0 0))