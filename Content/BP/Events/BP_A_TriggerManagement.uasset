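; Base trigger volume actor that fires an overridable Interaction event when the player's capsule enters its box while enabled.
; End chains triggers by enabling and disabling the actors in its activate and deactivate lists, then disables itself if flagged to run once.
; The construction script sizes and raises the box, sets its label text, and shows both only in debug mode.
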(event OnComponentBeginOverlap(TriggerBox)
  (params (OverlappedComponent :type Primitive%20Component%20Object%20Reference) (OtherActor :type Actor%20Object%20Reference) (OtherComp :type Primitive%20Component%20Object%20Reference) (OtherBodyIndex :type Integer) (bFromSweep :type Boolean) (SweepResult :type Hit%20Result%20Structure%20%28by%20ref%29))
  (bind _asbp_player (Utilities|Casting|CastToBP_Player OtherActor))
  (if (== OtherComp (Variables|/Script/Engine.Character|GetCapsuleComponent _asbp_player))
    (if (Variables|Enability|GetIsEnabled)
      (CallFunction|Interaction))))

(event Custom|SetBoxScale
  (Components|Box|SetBoxExtent (Variables|Default|GetTriggerBox) (Variables|Box|GetBoxScale) true)
  (Transformation|SetRelativeLocation (Variables|Default|GetTriggerBox) (Math|Vector|MakeVector 0.0 0.0 (.z (Variables|Box|GetBoxScale))) false false))

(event Custom|EnableTriggers
  (if (> (Utilities|Array|Length (Variables|Enability|GetTriggerToActivate)) 0)
    (for _array_element (Variables|Enability|GetTriggerToActivate)
      (Utilities|IsValid _array_element
        (:Is%20Valid
          (Variables|BP_A_TriggerManagement_C|SetIsEnabled _array_element true))))))

(event Custom|DisableTriggers
  (if (> (Utilities|Array|Length (Variables|Enability|GetTriggerToDeactivate)) 0)
    (for _array_element (Variables|Enability|GetTriggerToDeactivate)
      (Utilities|IsValid _array_element
        (:Is%20Valid
          (Variables|BP_A_TriggerManagement_C|SetIsEnabled _array_element false))))))

(event Custom|Interaction)

(event Custom|End
  (CallFunction|EnableTriggers)
  (CallFunction|DisableTriggers)
  (if (Variables|Enability|GetIsSaidOnce)
    (Variables|Enability|SetIsEnabled false)))

(event Custom|SetText
  (Rendering|Components|TextRender|SetText (Variables|Default|GetTextRender) (Variables|Box|GetText)))

(event Custom|SetDebug
  (bind _debugmode (Variables|Box|GetDebugMode))
  (bind _returnvalue (not _debugmode))
  (Development|SetHiddeninGame (Variables|Default|GetTriggerBox) _returnvalue false)
  (Development|SetHiddeninGame (Variables|Default|GetTextRender) _returnvalue false))

(fn ConstructionScript
  (|CallParentFunction)
  (CallFunction|SetBoxScale)
  (CallFunction|SetText)
  (CallFunction|SetDebug))