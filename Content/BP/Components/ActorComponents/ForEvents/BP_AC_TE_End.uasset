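; BP_AC_TE_End is an event actor component that ends the game when its UseEvent is triggered.
; UseEvent runs a custom event that disables controller movement and stops the character's background audio.
; After a short delay it calls End on a HUD widget, then waits longer and quits the game.
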(event Custom|CustomDelay
  (Variables|/Game/BP/Manager/BP_PC_MainPlayerController.BP_PC_MainPlayerController_C|SetCanMove (CallFunction|GetMyController) false)
  (Audio|Components|Audio|Stop (Variables|/Game/BP/Character/BP_Player.BP_Player_C|GetBackgroundAudio (CallFunction|GetMyCharacter)))
  (Utilities|FlowControl|Delay 2.0)
  (Default|End (Variables|/Game/BP/Components/ActorComponents/BP_AC_HUD.BP_AC_HUD_C|GetNewVar_0 (Variables|/Game/BP/Manager/BP_PC_MainPlayerController.BP_PC_MainPlayerController_C|GetBP_AC_HUD (CallFunction|GetMyController))))
  (Utilities|FlowControl|Delay 15.0)
  (Game|QuitGame 0 "Quit" false))

(event EventBeginPlay
  (|CallParentFunction))

(fn UseEvent
  (CallFunction|CustomDelay))