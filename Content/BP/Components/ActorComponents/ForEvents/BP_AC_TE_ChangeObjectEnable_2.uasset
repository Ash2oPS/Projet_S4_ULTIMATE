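; An event-driven actor component that enables or disables a list of target objects.
; On BeginPlay it puts each valid target in the inverse of the SetThemToVisible state, and UseEvent later applies that state.
; The shared SetVisible event calls SetSpawned on the target and switches its SkeletalMesh collision between query-and-physics and none.
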(event Custom|SetVisible
  (params (target :type BP%20Escargot%20Object%20Reference) (value :type Boolean))
  (Default|SetSpawned target value)
  (if value
    (Collision|SetCollisionEnabled (Variables|/Game/BP/Actors/BP_Escargot.BP_Escargot_C|GetSkeletalMesh target) "QueryAndPhysics")
    (else
      (Collision|SetCollisionEnabled (Variables|/Game/BP/Actors/BP_Escargot.BP_Escargot_C|GetSkeletalMesh target) "NoCollision"))))

(event EventBeginPlay
  (|CallParentFunction)
  (for _array_element (Variables|StaticMeshToModify|GetTargets)
    (Utilities|IsValid _array_element
      (:Is%20Valid
        (CallFunction|SetVisible _array_element (not (Variables|StaticMeshToModify|GetSetThemToVisible)))))))

(event EventTick
  (params (DeltaSeconds :type Float%20%28single-precision%29)))

(fn UseEvent
  (for _array_element (Variables|StaticMeshToModify|GetTargets)
    (Utilities|IsValid _array_element
      (:Is%20Valid
        (CallFunction|SetVisible _array_element (Variables|StaticMeshToModify|GetSetThemToVisible))))))