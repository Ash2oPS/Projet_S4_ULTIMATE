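; Event actor component that animates a door by rotating a referenced static mesh actor (Porte) when its UseEvent is called.
; UseEvent starts a configurable delay, then sets a flag that lets Tick drive the rotation.
; Tick lerps world rotation from the value cached at BeginPlay to Destination over one second, with optional shortest path.
; The timer is never reset, so the animation effectively plays only once.
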(event Custom|CustomDelay
  (Utilities|FlowControl|Delay (Variables|Default|GetWaitBeforePorte))
  (Variables|Default|SetisMoving true))

(event EventTick
  (params (DeltaSeconds :type Float%20%28single-precision%29))
  (if (Variables|Default|GetisMoving)
    (if (<= (Variables|Default|Gettimer) 1.0)
      (bind _output_get (Variables|Default|Settimer (+ DeltaSeconds (Variables|Default|Gettimer))))
      (Transformation|SetWorldRotation (Variables|/Script/Engine.StaticMeshActor|GetStaticMeshComponent (Variables|Default|GetPorte)) (Math|Rotator|Lerp(Rotator) (Variables|Default|GetBasRotation) (Variables|Default|GetDestination) _output_get (Variables|Default|GetShortest)) false false)
      (else
        (Variables|Default|SetisMoving false)))))

(event EventBeginPlay
  (|CallParentFunction)
  (Variables|Default|SetBasRotation (Transformation|GetWorldRotation (Variables|/Script/Engine.StaticMeshActor|GetStaticMeshComponent (Variables|Default|GetPorte)))))

(fn UseEvent
  (CallFunction|CustomDelay))