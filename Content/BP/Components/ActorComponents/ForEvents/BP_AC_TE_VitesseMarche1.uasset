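; BP_AC_TE_VitesseMarche1 is an event actor component that switches the post-process profile, despite a name suggesting walk speed.
; UseEvent finds the first BP_PostProcessManager in the level and, if valid, uses PPProfile to select one of its three enable functions: normal or two "PasNormal" variants.
; It contains no movement logic, and its BeginPlay is disabled.
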(event EventBeginPlay
  (|CallParentFunction) ; This node is disabled and will not be called.\nDrag off pins to build functionality.
)

(fn UseEvent
  (bind _outactors (Actor|GetAllActorsOfClass "/Game/BP/Manager/BP_PostProcessManager.BP_PostProcessManager_C"))
  (Utilities|IsValid (Utilities|Array|Get(acopy) _outactors)
    (:Is%20Valid
      (Variables|Default|SetPP_Manager (Utilities|Array|Get(acopy) _outactors))
      (switch int (Variables|Default|GetPP%20Profile)
        (:0
          (Default|EnablePPNormal (Variables|Default|GetPP_Manager)))
        (:1
          (Default|EnablePPPasNormal (Variables|Default|GetPP_Manager)))
        (:2
          (Default|EnabledPPPasNormal2 (Variables|Default|GetPP_Manager)))))))