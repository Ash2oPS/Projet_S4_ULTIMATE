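; BP_AC_TE_ChangeObjectEnable is an event component that shows or hides a set of target objects when its event is used.
; On BeginPlay it calls the parent, then sets each target's static mesh visibility to the opposite of SetThemToVisible.
; UseEvent applies SetThemToVisible to the same meshes, without propagating to children.
; Despite the "Enable" name, it changes only visibility.
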(event EventBeginPlay
  (|CallParentFunction)
  (for _array_element (Variables|StaticMeshToModify|GetTargets)
    (Rendering|SetVisibility (Variables|/Script/Engine.StaticMeshActor|GetStaticMeshComponent _array_element) (not (Variables|StaticMeshToModify|GetSetThemToVisible)) false)))

(event EventTick
  (params (DeltaSeconds :type Float%20%28single-precision%29)))

(fn UseEvent
  (for _array_element (Variables|StaticMeshToModify|GetTargets)
    (Rendering|SetVisibility (Variables|/Script/Engine.StaticMeshActor|GetStaticMeshComponent _array_element) (Variables|StaticMeshToModify|GetSetThemToVisible) false)))