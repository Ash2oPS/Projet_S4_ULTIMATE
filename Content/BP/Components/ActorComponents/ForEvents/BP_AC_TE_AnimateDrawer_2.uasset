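; Event actor component that slides drawer actors (Tiroirs) open or along an offset when triggered, with a sound.
; BeginPlay caches the first drawer's world position and adds it to Destination.
; UseEvent waits a delay, plays the sound there, then lets Tick lerp over Duration.
; Every drawer receives the same relative location, derived from that first drawer's world position.
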(event Custom|CustomDelay
  (Utilities|FlowControl|Delay (Variables|Default|GetWaitBeforeTiroir))
  (CallFunction|PlaySound)
  (Variables|Default|SetisMoving true))

(event Custom|PlaySound
  (Audio|PlaySoundatLocation (Variables|Default|GetDrawerSound) (Transformation|GetWorldLocation (Variables|/Script/Engine.Actor|GetRootComponent (Utilities|Array|Get(acopy) (Variables|Default|GetTiroirs)))) "0, 0, 0" 1.0 1.0 0.0 (Variables|Default|GetSoundAtten) 0 0))

(event EventTick
  (params (DeltaSeconds :type Float%20%28single-precision%29))
  (if (Variables|Default|GetisMoving)
    (if (<= (Variables|Default|Gettimer) 1.0)
      (bind _output_get (Variables|Default|Settimer (+ (/ DeltaSeconds (Variables|Default|GetDuration)) (Variables|Default|Gettimer))))
      (for _array_element (Variables|Default|GetTiroirs)
        (Transformation|SetRelativeLocation (Variables|/Script/Engine.Actor|GetRootComponent _array_element) (Math|Vector|Lerp(Vector) (Variables|Default|GetBasePosition) (Variables|Default|GetDestination) _output_get) false false))
      (else
        (Variables|Default|SetisMoving false)))))

(event EventBeginPlay
  (bind _tiroirs (Variables|Default|GetTiroirs))
  (bind _output (Utilities|Array|Get(acopy) _tiroirs))
  (|CallParentFunction)
  (Utilities|IsValid _output
    (:Is%20Valid
      (Variables|Default|SetBasePosition (Transformation|GetWorldLocation (Variables|/Script/Engine.Actor|GetRootComponent _output)))
      (Variables|Default|SetDestination (+ (Variables|Default|GetDestination) (Variables|Default|GetBasePosition))))))

(fn UseEvent
  (CallFunction|CustomDelay))