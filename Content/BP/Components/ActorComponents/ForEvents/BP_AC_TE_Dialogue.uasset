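; BP_AC_TE_Dialogue is an event component that plays a sequence of dialogue sentences with audio and subtitles when used.
; PlaySentence starts each sound and subtitle, using a fallback duration without audio, and returns its length plus a pause.
; MyDelay waits that time, advances the index and re-enters PlayDialogue until subtitles are removed.
; UnlocksWhenFinished decides whether the owning trigger's event ends immediately or after the last sentence.
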(event Custom|MyDelay
  (params (time :type Float%20%28single-precision%29))
  (Utilities|FlowControl|Delay time)
  (Math|Integer|IncrementInt (Variables|Dialogue|GetSentenceIndex)
    (:%20%20
      (CallFunction|PlayDialogue)
      (if (>= (Variables|Dialogue|GetSentenceIndex) (Utilities|Array|Length (Variables|Dialogue|GetSentences)))
        (CallFunction|RemoveSubtitles)
        (if (Variables|Dialogue|GetUnlocksWhenFinished)
          (Default|EndEvent (Variables|Default|GetBP_Trigger)))))))

(event EventBeginPlay
  (|CallParentFunction) ; This node is disabled and will not be called.\nDrag off pins to build functionality.
)

(event EventTick
  (params (DeltaSeconds :type Float%20%28single-precision%29)))

(fn UseEvent
  (CallFunction|PlayDialogue)
  (if (not (Variables|Dialogue|GetUnlocksWhenFinished))
    (Default|EndEvent (Variables|Default|GetBP_Trigger))))

(fn PlayDialogue
  (params (AudioSource :type Sound%20Attenuation%20Object%20Reference))
  (bind _sentences (Variables|Dialogue|GetSentences))
  (bind _returnvalue (Utilities|Array|Length _sentences))
  (if (> _returnvalue 0)
    (if (< (Variables|Dialogue|GetSentenceIndex) _returnvalue)
      (bind _delaytimer (CallFunction|PlaySentence AudioSource))
      (CallFunction|MyDelay _delaytimer)
      (else
        (CallFunction|RemoveSubtitles)))))

(fn PlaySentence
  (params (AudioSource :type Sound%20Attenuation%20Object%20Reference))
  (bind _sentenceindex (Variables|Dialogue|GetSentenceIndex))
  (bind _sentences (Variables|Dialogue|GetSentences))
  (bind _output (Utilities|Array|Get(acopy) _sentences _sentenceindex))
  (bind (_talkingcharacter _sentence _durationafternextsentence _audio) (Utilities|Struct|BreakBP_S_Replique _output))
  (Utilities|FlowControl|Sequence
    (:then_0
      ;[1 1 1] Check if there is an audio and sets duration
      (Utilities|IsValid _audio
        (:Is%20Valid
          (LocalVariables|SetAudioDuration (Variables|/Script/Engine.SoundBase|GetDuration _audio)))
        (:Is%20Not%20Valid
          (LocalVariables|SetAudioDuration 3.0)
          (LocalVariables|SetSubtitles (Utilities|Text|FormatText _sentence (Utilities|Text|MakeLiteralText " -NO AUDIO-"))))))
    (:then_1
      ;[1 1 1] Audio & Subtitles
      (CallFunction|CallSubtitles _sentence (LocalVariables|GetAudioDuration) _talkingcharacter)
      (Audio|PlaySoundatLocation _audio "0, 0, 0" "0, 0, 0" 1.0 1.0 0.0 0 0 0)
      (return (+ _durationafternextsentence (LocalVariables|GetAudioDuration))))))