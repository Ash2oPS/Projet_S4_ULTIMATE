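; Event actor component, named for a limping granny (MamieQuiBoite), that changes the player character's movement camera shake.
; UseEvent copies its three camera position variables into the three shake position slots of the character's BPCameraShakeOnMove.
; It has no other active logic: BeginPlay is disabled, and nothing here restores the previous shake positions.
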(event EventBeginPlay
  (|CallParentFunction) ; This node is disabled and will not be called.\nDrag off pins to build functionality.
)

(fn UseEvent
  (Variables|/Game/BP/Character/BP_CameraShakeOnMove.BP_CameraShakeOnMove_C|SetPositionCameraShake1 (Variables|/Game/BP/Character/BP_Player.BP_Player_C|GetBP_CameraShakeOnMove (CallFunction|GetMyCharacter)) (Variables|Default|GetCameraPos1))
  (Variables|/Game/BP/Character/BP_CameraShakeOnMove.BP_CameraShakeOnMove_C|SetPositionCameraShake2 (Variables|/Game/BP/Character/BP_Player.BP_Player_C|GetBP_CameraShakeOnMove (CallFunction|GetMyCharacter)) (Variables|Default|GetCameraPos2))
  (Variables|/Game/BP/Character/BP_CameraShakeOnMove.BP_CameraShakeOnMove_C|SetPositionCameraShake3 (Variables|/Game/BP/Character/BP_Player.BP_Player_C|GetBP_CameraShakeOnMove (CallFunction|GetMyCharacter)) (Variables|Default|GetCameraPos3)))