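; Event actor component that changes the material on a referenced static mesh actor when its UseEvent function is called.
; UseEvent applies NewMaterial to the configured material index, falls back to NewMaterialInstance if that is not valid, and does nothing if neither is set.
; BeginPlay only calls the parent implementation.
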(event EventBeginPlay
  (|CallParentFunction))

(fn UseEvent
  (Utilities|IsValid (Variables|ChangeMaterial|GetNewMaterial)
    (:Is%20Valid
      (Rendering|Material|SetMaterial (Variables|/Script/Engine.StaticMeshActor|GetStaticMeshComponent (Variables|ChangeMaterial|GetStaticMesh)) (Variables|ChangeMaterial|GetMaterialIndex) (Variables|ChangeMaterial|GetNewMaterial))
      (return))
    (:Is%20Not%20Valid
      (Utilities|IsValid (Variables|ChangeMaterial|GetNewMaterialInstance)
        (:Is%20Valid
          (Rendering|Material|SetMaterial (Variables|/Script/Engine.StaticMeshActor|GetStaticMeshComponent (Variables|ChangeMaterial|GetStaticMesh)) (Variables|ChangeMaterial|GetMaterialIndex) (Variables|ChangeMaterial|GetNewMaterialInstance))
          (return))
        (:Is%20Not%20Valid
          (return))))))