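; Actor component that launches an event when its owning BP_A_TriggerManagement actor fires its trigger.
; On BeginPlay it binds to the owner's EventToCall dispatcher.
; UseEventWithCondition compares the BoolCondition and IntCondition maps against global variables and calls UseEvent only if IsValid stays true, with no reset of that flag shown.
; UseEvent itself only prints a placeholder "Hello" message.
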(event EventBeginPlay
  (bind _asbp_a_trigger_management (Utilities|Casting|CastToBP_A_TriggerManagement (Components|GetOwner)))
  (EventDispatchers|BindEventtoEventtoCall _asbp_a_trigger_management (EventDispatchers|CreateEvent :!event UseEventwithCondition)))

(fn UseEvent
  (Development|PrintString "Hello"))

(fn UseEventwithCondition
  (Utilities|FlowControl|Sequence
    (:then_0
      (bind _keys (Utilities|Map|Keys (Variables|Default|GetBoolCondition)))
      (for _array_element _keys
        (if (Math|Boolean|NotEqual(Boolean) (Default|GetBoolValue (CallFunction|GetGlobalVariables) _array_element) (.Value (Utilities|Map|Find (Variables|Default|GetBoolCondition) _array_element)))
          (LocalVariables|SetIsValid false))))
    (:then_1
      (bind _keys_2 (Utilities|Map|Keys (Variables|Default|GetIntCondition)))
      (for _array_element_2 _keys_2
        (if (!= (Default|GetIntValue (CallFunction|GetGlobalVariables) _array_element_2) (.Value (Utilities|Map|Find (Variables|Default|GetIntCondition) _array_element_2)))
          (LocalVariables|SetIsValid false))))
    (:then_2
      (if (LocalVariables|GetIsValid)
        (CallFunction|UseEvent)))))