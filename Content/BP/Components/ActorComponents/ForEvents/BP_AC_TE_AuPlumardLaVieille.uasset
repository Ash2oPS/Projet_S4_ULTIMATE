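; Event actor component for the "AuPlumardLaVieille" event, which plays a day transition and relocates the player character.
; UseEvent starts the HUD's day transition, disables controller movement and calls CustomDelay.
; After a delay hidden behind the transition, CustomDelay snaps the character to a hardcoded position and rotation.
; A second delay then restores movement and switches the background audio to a creaky old house ambience.
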(event Custom|CustomDelay
  (bind _playercharacter (CallFunction|GetMyCharacter))
  (bind _backgroundaudio (Variables|/Game/BP/Character/BP_Player.BP_Player_C|GetBackgroundAudio _playercharacter))
  (bind _rootcomponent (Variables|/Script/Engine.Actor|GetRootComponent _playercharacter))
  (Utilities|FlowControl|Delay 4.0)
  (Transformation|SetWorldLocation _rootcomponent "-309.979370,725.269104,201.210281" false false)
  (Transformation|SetWorldRotation _rootcomponent "0,180.000000, 0" false false)
  (Utilities|FlowControl|Delay 5.0)
  (Variables|/Game/BP/Manager/BP_PC_MainPlayerController.BP_PC_MainPlayerController_C|SetCanMove (CallFunction|GetMyController) true)
  (Audio|Components|Audio|SetSound _backgroundaudio "/Game/Audio/BGM/393808__pfranzen__windy-creaky-old-house-ambience.393808__pfranzen__windy-creaky-old-house-ambience")
  (Audio|Components|Audio|Play _backgroundaudio 0.0))

(event EventBeginPlay
  (|CallParentFunction))

(fn UseEvent
  (bind _playercontroller (CallFunction|GetMyController))
  (Default|Transition (Variables|/Game/BP/Components/ActorComponents/BP_AC_HUD.BP_AC_HUD_C|GetDayTransitionHUD (Variables|/Game/BP/Manager/BP_PC_MainPlayerController.BP_PC_MainPlayerController_C|GetBP_AC_HUD _playercontroller)))
  (Variables|/Game/BP/Manager/BP_PC_MainPlayerController.BP_PC_MainPlayerController_C|SetCanMove _playercontroller false)
  (CallFunction|CustomDelay))