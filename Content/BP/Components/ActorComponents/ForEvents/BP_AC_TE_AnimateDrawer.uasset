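; Actor component for trigger events that slides drawer meshes open or to an offset position, with a positional sound.
; UseEvent waits a configurable delay, plays the sound, then Tick lerps world location over about one second.
; All meshes in Tiroirs share the start and destination computed from the first drawer at BeginPlay.
; UnlocksWhenFinished decides whether BPTrigger's event ends immediately or when the motion completes.
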(event Custom|CustomDelay
  (Utilities|FlowControl|Delay (Variables|Default|GetWaitBeforeTiroir))
  (CallFunction|PlaySound)
  (Variables|Default|SetisMoving true))

(event Custom|PlaySound
  (Audio|PlaySoundatLocation (Variables|Default|GetDrawerSound) (Transformation|GetWorldLocation (Variables|/Script/Engine.StaticMeshActor|GetStaticMeshComponent (Utilities|Array|Get(acopy) (Variables|Default|GetTiroirs)))) "0, 0, 0" 1.0 1.0 0.0 (Variables|Default|GetSoundAtten) 0 0))

(event EventTick
  (params (DeltaSeconds :type Float%20%28single-precision%29))
  (if (Variables|Default|GetisMoving)
    (if (<= (Variables|Default|Gettimer) 1.0)
      (bind _output_get (Variables|Default|Settimer (+ DeltaSeconds (Variables|Default|Gettimer))))
      (for _array_element (Variables|Default|GetTiroirs)
        (Transformation|SetWorldLocation (Variables|/Script/Engine.StaticMeshActor|GetStaticMeshComponent _array_element) (Math|Vector|Lerp(Vector) (Variables|Default|GetBasePosition) (Variables|Default|GetDestination) _output_get) false false))
      (else
        (Variables|Default|SetisMoving false)
        (if (Variables|Default|GetUnlocksWhenFinished)
          (Default|EndEvent (Variables|Default|GetBP_Trigger)))))))

(event EventBeginPlay
  (|CallParentFunction)
  (Variables|Default|SetBasePosition (Transformation|GetWorldLocation (Variables|/Script/Engine.StaticMeshActor|GetStaticMeshComponent (Utilities|Array|Get(acopy) (Variables|Default|GetTiroirs)))))
  (Variables|Default|SetDestination (+ (Variables|Default|GetDestination) (Variables|Default|GetBasePosition))))

(fn UseEvent
  (CallFunction|CustomDelay)
  (if (not (Variables|Default|GetUnlocksWhenFinished))
    (Default|EndEvent (Variables|Default|GetBP_Trigger))))