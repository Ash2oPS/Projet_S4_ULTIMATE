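; Main player controller for a first-person game, handling input, interaction, menus and the sleep-driven day change.
; Forwards movement and look axes to the character and triggers Interact on the selected item, all gated by CanMove.
; An optional per-tick camera line trace selects enabled BP_GInteractive_Item actors through their InteractionBox.
; Main, pause, options, credits and letter screens switch input mode, pause and cursor, with FlipFlops toggling main and pause menus.
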(event Custom|CustomTick)

(event Custom|Ouverture%20Lettre
  (Input|SetInputModeUIOnly self (Variables|/Game/BP/Components/ActorComponents/BP_AC_HUD.BP_AC_HUD_C|GetLetterHUD (Variables|Default|GetBP_AC_HUD)) "DoNotLock")
  (Game|SetGamePaused true)
  (Variables|Default|SetbShowMouseCursor true))

(event Custom|BoutonCrédits
  (Input|SetInputModeUIOnly (Game|GetPlayerController 0) 0 "DoNotLock")
  (bind _returnvalue (UserInterface|CreateWidget "/Game/BP/UI/WBP_CréditsMenu.WBP_CréditsMenu_C"))
  (bind _output_get (Variables|Default|SetWidgetCrédits _returnvalue))
  (UserInterface|Viewport|AddtoViewport _output_get 1000)
  (Game|SetGamePaused true)
  (Variables|Default|SetbShowMouseCursor true)
  (Widget|RemovefromParent (Variables|Default|GetWidgetMainMenu)))

(event Custom|MainMenu
  (bind _returnvalue (Game|GetPlayerController 0))
  (Utilities|FlowControl|FlipFlop
    (:A
      (Input|SetInputModeUIOnly _returnvalue 0 "DoNotLock")
      (bind _returnvalue_2 (UserInterface|CreateWidget "/Game/BP/UI/WBP_MainMenu.WBP_MainMenu_C"))
      (bind _output_get (Variables|Default|SetWidgetMainMenu _returnvalue_2))
      (UserInterface|Viewport|AddtoViewport _output_get 1000)
      (Game|SetGamePaused true)
      (Variables|Default|SetbShowMouseCursor true))
    (:B
      (Input|SetInputModeGameOnly _returnvalue)
      (Widget|RemovefromParent _output_get)
      (Game|SetGamePaused false)
      (Variables|Default|SetbShowMouseCursor false))))

(event Custom|BoutonOptionsRetour
  (Input|SetInputModeGameOnly (Game|GetPlayerController 0))
  (Widget|RemovefromParent (stale Custom|BoutonOptions _output_get))
  (Game|SetGamePaused true)
  (Variables|Default|SetbShowMouseCursor true)
  (UserInterface|Viewport|AddtoViewport (Variables|Default|GetWidgetMainMenu) 1000))

(event Custom|BoutonCréditsRetour
  (Input|SetInputModeGameOnly (Game|GetPlayerController 0))
  (Widget|RemovefromParent (stale Custom|BoutonCrédits _output_get))
  (Game|SetGamePaused true)
  (Variables|Default|SetbShowMouseCursor true)
  (UserInterface|Viewport|AddtoViewport (Variables|Default|GetWidgetMainMenu) 1000))

(event Custom|UpdatePostProcMedic
  ;[1 0 0] PostProcessManip
)

(event Custom|Sleep
  (Variables|Inputs|SetCanMove false)
  (bind _result (Math|Integer|IncrementInt (Math|Conversions|ToInteger(Byte) (Variables|TimeManager|GetCurrentDay)))
    (:%20%20
      (Variables|TimeManager|SetCurrentDay (Utilities|Enum|ByteToEnumBP_E_Days (Math|Conversions|ToByte(Integer) _result)))
      (Variables|Medicine|SetHasTakenMedicine false)
      (Variables|/Game/BP/Character/BP_Player.BP_Player_C|SetClosingEyes (Variables|Default|GetPlayer%20Character) true))))

(event Custom|Pause/Unpause%20Game
  (bind _returnvalue (Game|GetPlayerController 0))
  (Utilities|FlowControl|FlipFlop
    (:A
      (Input|SetInputModeUIOnly _returnvalue 0 "DoNotLock")
      (bind _returnvalue_2 (UserInterface|CreateWidget "/Game/BP/UI/WBP_PauseMenu.WBP_PauseMenu_C"))
      (bind _output_get (Variables|Default|SetWidgetPause _returnvalue_2))
      (UserInterface|Viewport|AddtoViewport _output_get 1000)
      (Game|SetGamePaused true)
      (Variables|Default|SetbShowMouseCursor true))
    (:B
      (Input|SetInputModeGameOnly _returnvalue)
      (Widget|RemovefromParent _output_get)
      (Game|SetGamePaused false)
      (Variables|Default|SetbShowMouseCursor false))))

(event Custom|SetHasToRaycast
  (params (value :type Boolean))
  (Variables|Default|SetHasToRaycast value))

(event Custom|Fermeture%20Lettre
  (Input|SetInputModeGameOnly self)
  (Game|SetGamePaused false)
  (Variables|Default|SetbShowMouseCursor false))

(event Custom|BoutonOptions
  (Input|SetInputModeUIOnly (Game|GetPlayerController 0) 0 "DoNotLock")
  (bind _returnvalue (UserInterface|CreateWidget "/Game/BP/UI/WBP_OptionsMenu.WBP_OptionsMenu_C"))
  (bind _output_get (Variables|Default|SetWidgetOptions _returnvalue))
  (UserInterface|Viewport|AddtoViewport _output_get 1000)
  (Game|SetGamePaused true)
  (Variables|Default|SetbShowMouseCursor true)
  (Widget|RemovefromParent (Variables|Default|GetWidgetMainMenu)))

(event EventBeginPlay
  ;[0.3986 1 0.1379] BeginPlay
  (Utilities|FlowControl|Sequence
    (:then_0
      ;;[1 1 1] Create UI
      (bind _returnvalue (UserInterface|CreateWidget "/Game/BP/UI/WBP_InteractTo.WBP_InteractTo_C" self))
      (bind _output_get (Variables|Default|SetInteractUI _returnvalue))
      (UserInterface|Viewport|AddtoViewport _output_get 0))
    (:then_1
      ;;[1 1 1] Getters
      (bind _returnvalue_2 (Actor|GetActorOfClass "/Script/Engine.PostProcessVolume"))
      (Variables|Default|SetPostProcVol _returnvalue_2)
      (Variables|Default|SetPlayer%20Character (CallFunction|GetMyCharacter)))
    (:then_2
      (CallFunction|MainMenu))))

(event EventTick
  (params (DeltaSeconds :type Float%20%28single-precision%29))
  ;[0 0.3464 1] EventTick
  (Utilities|FlowControl|Sequence
    (:then_0
      (if (Variables|Default|GetHasToRaycast)
        (CallFunction|RaycastThings)))
    (:then_2
      (CallFunction|CustomTick))))

(event Input|ActionEvents|InputActionInteract
  (params (Key :type Key%20Structure :default "None"))
  (:Pressed
    (if (Variables|Inputs|GetCanMove)
      (Utilities|IsValid (Variables|Default|GetSelectedObject)
        (:Is%20Valid
          (Default|Interaction (Variables|Default|GetSelectedObject)))))))

(event Input|ActionEvents|InputActionPauseMenu
  (params (Key :type Key%20Structure :default "None"))
  (:Pressed
    (CallFunction|Pause/UnpauseGame)))

(event Input|ActionEvents|InputActionSkip
  (params (Key :type Key%20Structure :default "None"))
  (:Pressed
    (Default|CallSkipDispatcher)))

(event Input|AxisEvents|InputAxisMoveRight
  (params (AxisValue :type Float%20%28single-precision%29))
  (if (Variables|Inputs|GetCanMove)
    (Default|AxisMoveRIght (Variables|Default|GetPlayer%20Character) AxisValue)))

(event Input|AxisEvents|InputAxisMoveForward
  (params (AxisValue :type Float%20%28single-precision%29))
  (if (Variables|Inputs|GetCanMove)
    (Default|AxisMoveForward (Variables|Default|GetPlayer%20Character) AxisValue)))

(event Input|AxisEvents|InputAxisTurn
  (params (AxisValue :type Float%20%28single-precision%29))
  (if (Variables|Inputs|GetCanMove)
    (Default|AxisTurn (Variables|Default|GetPlayer%20Character) AxisValue)))

(event Input|AxisEvents|InputAxisLookUp
  (params (AxisValue :type Float%20%28single-precision%29))
  (if (Variables|Inputs|GetCanMove)
    (Default|AxisLookUp (Variables|Default|GetPlayer%20Character) AxisValue)))

(event Input|AxisEvents|InputAxisLookUpRate
  (params (AxisValue :type Float%20%28single-precision%29))
  (if (Variables|Inputs|GetCanMove)
    (Default|AxisLookUpRate (Variables|Default|GetPlayer%20Character) AxisValue)))

(event Input|AxisEvents|InputAxisTurnRate
  (params (AxisValue :type Float%20%28single-precision%29))
  (if (Variables|Inputs|GetCanMove)
    (Default|AxisTurnRate (Variables|Default|GetPlayer%20Character) AxisValue)))

(fn ConstructionScript)

(fn RaycastThings
  (bind _player_character (Variables|Default|GetPlayer%20Character))
  (bind _firstpersoncamera (Variables|/Game/BP/Character/BP_Player.BP_Player_C|GetFirstPersonCamera _player_character))
  (bind _returnvalue (Transformation|GetWorldLocation _firstpersoncamera))
  ;[0.3551 1 0.6655] Raycast
  (bind _outhit (Class|KismetSystemLibrary|LineTraceSinglebyProfile _returnvalue (+ _returnvalue (* (Math|Vector|GetForwardVector _firstpersoncamera) (Variables|Controls|GetGrabDistance))) "EnabledTrig" false 0 "None" true))
  (Utilities|IsValid (.HitActor (Collision|BreakHitResult _outhit))
    (:Is%20Valid
      ;[1 1 1] Raycast To Bp_Interactive
      (bind _asbp_ginteractive_item (Utilities|Casting|CastToBP_GInteractive_Item (.HitActor (Collision|BreakHitResult _outhit)))
        (:then
          ;;[0.5431 1 0.2257] Selection
          (if (== (.HitComponent (Collision|BreakHitResult _outhit)) (Variables|/Game/BP/Events/CeuxQuiNousInteressent/BP_GInteractive_Item.BP_GInteractive_Item_C|GetInteractionBox _asbp_ginteractive_item))
            (Utilities|IsValid (Variables|Default|GetSelectedObject)
              (:Is%20Not%20Valid
                (if (Variables|/Game/BP/Events/BP_A_TriggerManagement.BP_A_TriggerManagement_C|GetIsEnabled _asbp_ginteractive_item)
                  (bind _output_get (Variables|Default|SetSelectedObject _asbp_ginteractive_item))
                  (Default|OnSelected _output_get))))))
        (:CastFailed
          ;;[1 0.277 0.7133] Unselection
          (Utilities|IsValid (Variables|Default|GetSelectedObject)
            (:Is%20Valid
              (Default|OnUnselected (Variables|Default|GetSelectedObject))
              (Variables|Default|SetSelectedObject 0))))))))