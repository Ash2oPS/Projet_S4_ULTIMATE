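; BP_PostProcessManager switches the game's post-process look between three presets: one normal and two "PasNormal" (not normal) variants.
; Three events each enable one of PPNormal, PPPasNormal or PPPasNormal2 and disable the other two, so each call leaves a single preset active.
; The switch is a plain toggle of each Enabled flag with no blending, and the file itself never calls these events.
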(event Custom|EnablePP_Normal
  (Variables|/Script/Engine.PostProcessVolume|SetbEnabled (Variables|Default|GetPP_Normal) true)
  (Variables|/Script/Engine.PostProcessVolume|SetbEnabled (Variables|Default|GetPP_PasNormal) false)
  (Variables|/Script/Engine.PostProcessVolume|SetbEnabled (Variables|Default|GetPP_PasNormal2) false))

(event Custom|EnablePP_PasNormal
  (Variables|/Script/Engine.PostProcessVolume|SetbEnabled (Variables|Default|GetPP_Normal) false)
  (Variables|/Script/Engine.PostProcessVolume|SetbEnabled (Variables|Default|GetPP_PasNormal) true)
  (Variables|/Script/Engine.PostProcessVolume|SetbEnabled (Variables|Default|GetPP_PasNormal2) false))

(event Custom|EnabledPP_PasNormal2
  (Variables|/Script/Engine.PostProcessVolume|SetbEnabled (Variables|Default|GetPP_Normal) false)
  (Variables|/Script/Engine.PostProcessVolume|SetbEnabled (Variables|Default|GetPP_PasNormal) false)
  (Variables|/Script/Engine.PostProcessVolume|SetbEnabled (Variables|Default|GetPP_PasNormal2) true))

(fn ConstructionScript)