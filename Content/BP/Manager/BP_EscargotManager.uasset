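; Manager that registers every BP_Escargot (snail) in the level, randomizes its look and can hide groups of them.
; On BeginPlay it assigns each snail an ID and manager reference, randomizes material, per-axis scale and animation rate, and rarely makes one gold.
; Snails added to the visible list by ID are later despawned together by disabling visibility and collision rather than destroying them, then clearing the list.
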(event Custom|AddEscargotToVisibles
  (params (ID :type Integer))
  (bind _touslesescargots (Variables|Default|GetTousLesEscargots))
  (bind (_value _returnvalue) (Utilities|Map|Find _touslesescargots ID))
  (if _returnvalue
    (Utilities|Array|Add (Variables|Default|GetLesEsargotsVisibles) _value)))

(event Custom|DespawnEscargotVisibles
  (for _array_element (Variables|Default|GetLesEsargotsVisibles)
    (Rendering|SetVisibility (Variables|/Game/BP/Actors/BP_Escargot.BP_Escargot_C|GetSkeletalMesh _array_element) false false)
    (Collision|SetCollisionEnabled (Variables|/Game/BP/Actors/BP_Escargot.BP_Escargot_C|GetSkeletalMesh _array_element) "NoCollision"))
  (Utilities|Array|Clear (Variables|Default|GetLesEsargotsVisibles)))

(event EventBeginPlay
  (bind _returnvalue (Math|Float|MakeLiteralFloat 0.8))
  (bind _returnvalue_2 (Math|Float|MakeLiteralFloat 1.2))
  (bind _materials (Variables|Default|GetMaterials))
  (bind _returnvalue_3 (Math|Random|RandomFloatinRange _returnvalue _returnvalue_2))
  (bind _outactors (Actor|GetAllActorsOfClass "/Game/BP/Actors/BP_Escargot.BP_Escargot_C"))
  (for (_array_element _array_index) _outactors
    (Utilities|Map|Add (Variables|Default|GetTousLesEscargots) _array_index _array_element)
    (Variables|/Game/BP/Actors/BP_Escargot.BP_Escargot_C|SetEscargotID _array_element _array_index)
    (Variables|/Game/BP/Actors/BP_Escargot.BP_Escargot_C|SetManager _array_element self)
    (Rendering|Material|SetMaterial (Variables|/Game/BP/Actors/BP_Escargot.BP_Escargot_C|GetSkeletalMesh _array_element) 0 (Utilities|Array|Get(acopy) _materials (Math|Random|RandomInteger (Utilities|Array|Length _materials))))
    (Transformation|SetRelativeScale3D (Variables|/Game/BP/Actors/BP_Escargot.BP_Escargot_C|GetSkeletalMesh _array_element) (Math|Vector|MakeVector _returnvalue_3 _returnvalue_3 _returnvalue_3))
    (Components|Timeline|SetPlayRate (Variables|/Game/BP/Actors/BP_Escargot.BP_Escargot_C|GetSkeletalMesh _array_element) (Math|Random|RandomFloatinRange (Math|Float|MakeLiteralFloat 0.8) (Math|Float|MakeLiteralFloat 1.2)))
    (if (== (Math|Random|RandomInteger 60) 59)
      (Variables|/Game/BP/Actors/BP_Escargot.BP_Escargot_C|SetGold _array_element true)
      (Rendering|Material|SetMaterial (Variables|/Game/BP/Actors/BP_Escargot.BP_Escargot_C|GetSkeletalMesh _array_element) 0 "/Game/Game_Art/Anime/Escargot/m_escargot_Gold.m_escargot_Gold"))))

(fn ConstructionScript)