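; Camera shake Blueprint that sways the view by adding yaw and pitch input to its owner's Instigator.
; Tick advances a looping timer with delta seconds, splits it at two time points, and applies one of three fixed offsets each frame.
; Its gate compares constants, so the shake runs every tick regardless of movement.
; Sine/cosine and vector-lerp variants remain as unused nodes.
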(event EventBeginPlay)

(event EventTick
  (params (DeltaSeconds :type Float%20%28single-precision%29))
  (bind _returnvalue (Components|GetOwner))
  (bind _positioncamerashake1 (Variables|Default|GetPositionCameraShake1))
  (bind _positioncamerashake2 (Variables|Default|GetPositionCameraShake2))
  (bind _positioncamerashake3 (Variables|Default|GetPositionCameraShake3))
  (bind _instigator (Variables|/Script/Engine.Actor|GetInstigator _returnvalue))
  (if (not (== 1.0 0.0))
    (Variables|Default|SetWalkingLoopParameter (+ (Variables|Default|GetWalkingLoopParameter) (Utilities|Time|GetWorldDeltaSeconds)))
    (if (< (Variables|Default|GetWalkingLoopParameter) (Variables|Default|GetPointCamera1))
      (Pawn|Input|AddControllerYawInput _instigator (.x _positioncamerashake1))
      (Pawn|Input|AddControllerPitchInput _instigator (.y _positioncamerashake1))
      (elif (< (Variables|Default|GetWalkingLoopParameter) (Variables|Default|GetPointCamera2))
        (Pawn|Input|AddControllerYawInput _instigator (.x _positioncamerashake2))
        (Pawn|Input|AddControllerPitchInput _instigator (.y _positioncamerashake2))
        (else
          (Pawn|Input|AddControllerYawInput _instigator (.x _positioncamerashake3))
          (Pawn|Input|AddControllerPitchInput _instigator (.y _positioncamerashake3)))))
    (if (> (Variables|Default|GetWalkingLoopParameter) (Variables|Default|GetLoopLength))
      (Variables|Default|SetWalkingLoopParameter 0.0))))